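; Player controller that turns Enhanced Input actions into movement, camera look and spell casting for the controlled pawn.
; Move input follows control rotation and snaps the pawn's yaw to the camera's, while look input feeds yaw and pitch.
; Starting fire input attaches a Niagara ring of flames to the BP_Character mesh, removed on cancel or completion.
; Completion also spawns BP_Spell_Launch at an offset rotated with the pawn and sets the character as its owner.
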(event Input|EnhancedActionEvents|EnhancedInputActionIA_Move
  (params (ActionValue :type Vector%202D%20Structure) (ElapsedSeconds :type Float%20%28double-precision%29) (TriggeredSeconds :type Float%20%28double-precision%29) (InputAction :type Input%20Action%20Object%20Reference :default "/Game/_GameManager/Inputs/IA_Move.IA_Move"))
  (bind _returnvalue (Pawn|GetControlRotation :!class /Script/Engine.Controller))
  (bind (_x _y) (Math|Vector2D|BreakVector2D ActionValue))
  (bind _returnvalue_2 (Pawn|GetControlledPawn))
  (bind _returnvalue_3 (Transformation|GetActorRotation _returnvalue_2))
  (bind (_roll _pitch) (Math|Rotator|BreakRotator _returnvalue_3))
  (Pawn|Input|AddMovementInput (Pawn|GetControlledPawn) (Math|Vector|GetForwardVector (Math|Rotator|MakeRotator 0.0 0.0 (.yaw (Pawn|GetControlRotation :!class /Script/Engine.Controller)))) _y false)
  (Pawn|Input|AddMovementInput (Pawn|GetControlledPawn) (Math|Vector|GetRightVector (Math|Rotator|MakeRotator (.roll _returnvalue) 0.0 (.yaw _returnvalue))) _x false)
  ;[0.35 0.45 1] Rotate Player Forward To Camera Forward
  (Transformation|SetActorRelativeRotation _returnvalue_2 (Math|Rotator|MakeRotator _roll _pitch (.yaw (Variables|/Script/Engine.SceneComponent|GetRelativeRotation (Variables|/Script/Engine.PlayerCameraManager|GetTransformComponent (Game|GetPlayerCameraManager 0))))) true))

(event Input|EnhancedActionEvents|EnhancedInputActionIA_Look
  (params (ActionValue :type Vector%202D%20Structure) (ElapsedSeconds :type Float%20%28double-precision%29) (TriggeredSeconds :type Float%20%28double-precision%29) (InputAction :type Input%20Action%20Object%20Reference :default "/Game/_GameManager/Inputs/IA_Look.IA_Look"))
  (bind (_x _y) (Math|Vector2D|BreakVector2D ActionValue))
  (Class|PlayerController|AddYawInput _x)
  (Class|PlayerController|AddPitchInput _y))

(event Input|EnhancedActionEvents|EnhancedInputActionIA_FireInput
  (params (ActionValue :type Boolean) (ElapsedSeconds :type Float%20%28double-precision%29) (TriggeredSeconds :type Float%20%28double-precision%29) (InputAction :type Input%20Action%20Object%20Reference :default "/Game/_GameManager/Inputs/IA_FireInput.IA_FireInput"))
  (bind _returnvalue (Pawn|GetControlledPawn))
  (bind _returnvalue_2 (Transformation|GetActorTransform _returnvalue))
  (bind _asbp_character (Utilities|Casting|CastToBP_Character _returnvalue))
  (:Started
    (bind _returnvalue_3 (Niagara|SpawnSystemAttached "/Game/MegaMagicVFXBundle/VFX/MagicAuraVFX/VFX/RingOfFlames/Systems/N_RingOfFlames.N_RingOfFlames" (Variables|/Script/Engine.Character|GetMesh _asbp_character) "Socket" "0, 0, 0" "90.000000,0.000000,0.000000" "KeepRelativeOffset" false)))
  (:Canceled
    (Components|DestroyComponent _returnvalue_3))
  (:Completed
    (Components|DestroyComponent _returnvalue_3)
    (bind _returnvalue_4 (Game|SpawnActorfromClass "/Game/Spells/BP_Spell_Launch.BP_Spell_Launch_C" (Math|Transform|MakeTransform (+ (.location _returnvalue_2) (Math|Vector|RotateVector "50.000000,20.000000,20.000000" (Transformation|GetActorRotation _returnvalue))) (.rotation _returnvalue_2) (.scale _returnvalue_2)) "Undefined" "MultiplyWithRoot" 0 0))
    (Variables|/Game/Spells/BP_Spell_Launch.BP_Spell_Launch_C|SetOwnerChar _returnvalue_4 _asbp_character)))

(event Input|EnhancedActionEvents|EnhancedInputActionIA_Sprint
  (params (ActionValue :type Boolean) (ElapsedSeconds :type Float%20%28double-precision%29) (TriggeredSeconds :type Float%20%28double-precision%29) (InputAction :type Input%20Action%20Object%20Reference :default "/Game/_GameManager/Inputs/IA_Sprint.IA_Sprint")))

(event EventBeginPlay)

(event EventTick
  (params (DeltaSeconds :type Float%20%28single-precision%29)))

(fn ConstructionScript)